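; Sea-life spawner actor that spawns one randomly chosen AI fish from the FishToSpawn class array at BeginPlay.
; The spawn point is the actor's location with a random X and Y offset, keeping the same Z.
; A chain of range checks picks among seven array entries, looping back if none match.
; Each check rolls a fresh random number, so the selection odds are uneven.
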(event `self.ReceiveBeginPlay`
  (bind _returnvalue (`KismetMathLibrary.RandomIntegerInRange` 0 70))
  (bind (_returnvalue_x _returnvalue_y _returnvalue_z) (`KismetMathLibrary.BreakVector` (`self.K2_GetActorLocation`)))
  (bind _returnvalue_2 (`KismetMathLibrary.RandomFloatInRange` 50.0 20.0))
  ;[0 0.0357 1] Fish_Spawn_Location
  (set `self.FishSpawnLocation` (`KismetMathLibrary.MakeVector` (+ _returnvalue_x _returnvalue_2) (+ _returnvalue_y _returnvalue_2) _returnvalue_z))
  ;[1 0 0.6034] Fish_Spawn_Type
  (if (< _returnvalue 10) :!label _label
    (`AIBlueprintHelperLibrary.SpawnAIFromClass` (`|GetArrayItem` (`self.FishToSpawn`)) null (`self.FishSpawnLocation`) (struct) false null)
    (elif (and (>= _returnvalue 10) (< _returnvalue 20))
      (`AIBlueprintHelperLibrary.SpawnAIFromClass` (`|GetArrayItem` (`self.FishToSpawn`) 1) null (`self.FishSpawnLocation`) (struct) false null)
      (elif (and (>= _returnvalue 20) (< _returnvalue 30))
        (`AIBlueprintHelperLibrary.SpawnAIFromClass` (`|GetArrayItem` (`self.FishToSpawn`) 2) null (`self.FishSpawnLocation`) (struct) false null)
        (elif (and (>= _returnvalue 30) (< _returnvalue 40))
          (`AIBlueprintHelperLibrary.SpawnAIFromClass` (`|GetArrayItem` (`self.FishToSpawn`) 3) null (`self.FishSpawnLocation`) (struct) false null)
          (elif (and (>= _returnvalue 40) (< _returnvalue 50))
            (`AIBlueprintHelperLibrary.SpawnAIFromClass` (`|GetArrayItem` (`self.FishToSpawn`) 4) null (`self.FishSpawnLocation`) (struct) false null)
            (elif (and (>= _returnvalue 50) (< _returnvalue 60))
              (`AIBlueprintHelperLibrary.SpawnAIFromClass` (`|GetArrayItem` (`self.FishToSpawn`) 5) null (`self.FishSpawnLocation`) (struct) false null)
              (elif (>= _returnvalue 60)
                (`AIBlueprintHelperLibrary.SpawnAIFromClass` (`|GetArrayItem` (`self.FishToSpawn`) 6) null (`self.FishSpawnLocation`) (struct) false null)
                (else
                  (goto _label))))))))))

(fn `UserConstructionScript`)