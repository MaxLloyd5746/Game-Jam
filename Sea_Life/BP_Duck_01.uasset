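; BP_Duck_01 is a duck AI character that follows the player.
; On BeginPlay it starts an AI move toward the player character, repeating after a short delay only when the move succeeds; failure is not handled.
; GetPathRoute exposes a stored route, and SetMoveSpeed maps movement states such as Idle or Panicked to walk speeds, though neither is called in this graph.
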(event `self.ReceiveBeginPlay`
  ;[1 1 1] Enemy Movement
  (`self.FollowPlayer`))

(event `FollowPlayer`
  ;[1 1 1] Enemy Movement
  (`|AIMoveTo` self (0.0 0.0 0.0) (`GameplayStatics.GetPlayerCharacter` 0) 200.0
    (:`OnSuccess`
      (`KismetSystemLibrary.Delay` 5.0)
      (`self.FollowPlayer`))))

(fn `GetPathRoute`
  (returns (PathRoute :type "/Game/Sea_Life/AI/BP_Fish_Movement Object Reference"))
  (return (`self.PathRoute`)))

(fn `SetMoveSpeed`
  (params (Speed :type "/Game/Sea_Life/AI/Enums/E_Movement_Speed Enum" :default "NewEnumerator0"))
  (returns (`Speed Value` :type "Float (double-precision)"))
  (bind _output_get (set `CharacterMovementComponent.MaxWalkSpeed` (select `/Game/Sea_Life/AI/Enums/E_Movement_Speed` Speed :`NewEnumerator0` 200.0 :`NewEnumerator1` 600.0 :`NewEnumerator2` 400.0 :`NewEnumerator3` 100.0 :!type "Float (single-precision)") (`self.CharacterMovement`)))
  (return _output_get))

(fn `UserConstructionScript`)